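; MyPlayerState is a player state Blueprint that stores a player's team name, ship choice and pawn reference.
; The SelectTeam, SelectShip and Setpawn events each write one of these variables.
; Matching getter functions return the stored values, and BeginPlay, Tick and the construction script do nothing.
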(event Custom|Select%20Ship
  (params (SelectedShip :type Character%20Class%20Reference))
  (Variables|Default|SetShipChoice SelectedShip))

(event Custom|Select%20Team
  (params (TeamName :type String))
  (Variables|Default|SetTeamName TeamName))

(event Custom|Set%20pawn
  (params (Pawn :type My%20Spectator%20Pawn%20Object%20Reference))
  (Variables|Default|SetPawnReference Pawn))

(event EventBeginPlay)

(event EventTick
  (params (DeltaSeconds :type Float%20%28single-precision%29)))

(fn ConstructionScript)

(fn GetShipChoice
  (return (Variables|Default|GetShipChoice)))

(fn GetTeamName
  (return (Variables|Default|GetTeamName)))

(fn GetPawnReference
  (return (Variables|Default|GetPawnReference)))