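; CustomPlayerController is a player controller Blueprint that links itself to the game instance and caches its player state.
; On BeginPlay it casts the game instance to MyGameInstance, stores it and registers itself through AddSelf.
; It then casts its PlayerState to MyPlayerState and stores it, exposed through the GetMyPlayerstate getter.
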(event EventBeginPlay
  (bind _asmy_game_instance (Utilities|Casting|CastToMyGameInstance (Game|GetGameInstance)))
  (bind _output_get (Variables|Default|SetGameInstance _asmy_game_instance))
  (Default|AddSelf _output_get self)
  (bind _asmy_player_state (Utilities|Casting|CastToMyPlayerState (Variables|Default|GetPlayerState)))
  (Variables|Default|SetMyPlayerState _asmy_player_state))

(fn ConstructionScript)

(fn GetMyPlayerstate
  (return (Variables|Default|GetMyPlayerState)))