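; Spectator pawn that serves as a placeholder until a player's chosen character is spawned.
; On BeginPlay it disables input for player controller 0 and registers itself as the pawn on MyPlayerState.
; SpawnInPlayer spawns the chosen class at a given transform, even if colliding, has the supplied controller possess it, then destroys the spectator.
; The construction script caches a MyGameInstance reference, which the shown graphs never use.
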(event Custom|SpawnInPlayer
  (params (ChosenPlayer :type Character%20Class%20Reference) (Location :type Transform) (PC :type Player%20Controller%20Object%20Reference))
  (bind _returnvalue (Game|SpawnActorfromClass ChosenPlayer Location true 0))
  (Pawn|Possess PC _returnvalue)
  (Actor|DestroyActor))

(event EventActorBeginOverlap
  (params (OtherActor :type Actor%20Object%20Reference)))

(event EventTick
  (params (DeltaSeconds :type Float%20%28single-precision%29)))

(event EventBeginPlay
  (Input|DisableInput (Game|GetPlayerController 0))
  (CallFunction|SetPawntoInstance))

(fn ConstructionScript
  (bind _asmy_game_instance (Utilities|Casting|CastToMyGameInstance (Game|GetGameInstance)))
  (Variables|Default|SetGameInstance _asmy_game_instance))

(fn SetPawntoInstance
  (bind _asmy_player_state (Utilities|Casting|CastToMyPlayerState (Variables|GetPlayerState)))
  (Default|SetPawn _asmy_player_state self))